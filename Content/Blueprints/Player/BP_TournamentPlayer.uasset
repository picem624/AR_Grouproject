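; Player Blueprint for a tournament-management UI that creates the main HUD and acts as its VaRest client to a localhost API.
; It handles user registration, login, and team and tournament registration, with callbacks updating HUD widgets.
; Bearer tokens authorize tournament creation; a 403 triggers token refresh, which replays the pending action or shows the login screen.
; Team registrations save to the MyGame slot, while the tournament save nodes are disconnected.
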(event `self.ReceiveBeginPlay`
  (bind _returnvalue (`|CreateWidget` "/Game/widgets/Tournament/MainHud.MainHud_C"))
  (bind _output_get (set `self.HudRef` _returnvalue))
  (`UserWidget.AddToViewport` _output_get 0)
  (`WidgetBlueprintLibrary.SetInputMode_UIOnlyEx` (`GameplayStatics.GetPlayerController` 0) _output_get))

(event `Register`
  (bind _returnvalue (`VaRestRequestJSON.GetRequestObject` (`self.Json Post Object`)))
  ;[0 0 0 1 50] Registrate
  ;;[1 1 1] make Json Request
  (bind _returnvalue_2 (`VaRestSubsystem.ConstructVaRestRequestExt` (subsystem `VaRestSubsystem`) "POST" "json"))
  (bind _output_get (set `self.Json Post Object` _returnvalue_2))
  (add `VaRestRequestJSON.OnRequestComplete` _output_get (delegate `eventSuccess`))
  (add `VaRestRequestJSON.OnRequestFail` _output_get (delegate `eventfailed`))
  ;;[1 1 1] set variables inJSON Object
  (`VaRestJsonObject.SetStringField` _returnvalue "username" (`self.username`))
  (`VaRestJsonObject.SetStringField` _returnvalue "password" (`self.password`))
  (`VaRestJsonObject.SetObjectField` _returnvalue "contactData" (`|MakeJson` (`self.FirstName`) (`self.Surename`) (`self.Email`) (`self.Phone Number`)))
  (`VaRestRequestJSON.SetRequestObject` (`self.Json Post Object`) _returnvalue)
  (`VaRestRequestJSON.ProcessURL` (`self.Json Post Object`) "http://localhost:8080/api/register"))

(event `eventfailed`
  (params (Request :type "VaRestRequestJSON Object Reference"))
  ;[0 0 0 1 50] Registrate
  (`KismetSystemLibrary.PrintString` "failed"))

(event `eventSuccess`
  (params (Request :type "VaRestRequestJSON Object Reference"))
  (bind _alreadyusedinfo (`/Game/widgets/Tournament/Register.alreadyUsedInfo` (`/Game/widgets/Tournament/MainHud.Register` (`self.HudRef`))))
  ;[0 0 0 1 50] Registrate
  (bind _returnvalue (`VaRestRequestJSON.GetResponseContentAsString` Request true))
  (if (`KismetStringLibrary.EqualEqual_StrStr` (`KismetStringLibrary.GetSubstring` _returnvalue 5 9) "duplicate")
    ;;[1 1 1] if duplicate was true. show error message in widget
    (`TextBlock.SetText` _alreadyusedinfo "this name is already in use")
    (`TextBlock.SetColorAndOpacity` _alreadyusedinfo (make `SlateColor` (struct :`R` 1.0 :`B` 0.016462 :`A` 1.0)))
    (else
      (`KismetSystemLibrary.PrintString` _returnvalue))))

(event `Login`
  ;[0 0 0 1 40] Login
  (bind _returnvalue (`VaRestSubsystem.ConstructVaRestRequestExt` (subsystem `VaRestSubsystem`) "POST" "json"))
  (bind _output_get (set `self.Json Post Object` _returnvalue))
  (bind _returnvalue_2 (`VaRestRequestJSON.GetRequestObject` _output_get))
  ;;[1 1 1] Set fields in json object
  (`VaRestJsonObject.SetStringField` _returnvalue_2 "username" (`self.username`))
  (`VaRestJsonObject.SetStringField` _returnvalue_2 "password" (`self.password`))
  (add `VaRestRequestJSON.OnRequestComplete` _output_get (delegate `GetBearerToken`))
  (add `VaRestRequestJSON.OnRequestFail` _output_get (delegate `AuthorizationFailed`))
  (`VaRestRequestJSON.ProcessURL` (`self.Json Post Object`) "http://localhost:8080/api/login"))

(event `AuthorizationFailed`
  (params (Request :type "VaRestRequestJSON Object Reference"))
  ;[0 0 0 1 40] Login
)

(event `GetBearerToken`
  (params (Request :type "VaRestRequestJSON Object Reference"))
  (bind _returnvalue (`VaRestRequestJSON.GetResponseObject` Request))
  ;[0 0 0 1 40] Login
  ;;[1 1 1] If login successful, get the access and refresh token
  (if (== (`VaRestRequestJSON.GetResponseCode` Request) 401)
    (`KismetSystemLibrary.PrintString` "invalid username or Password")
    (else
      (set `self.Bearer token` (`VaRestJsonObject.GetStringField` _returnvalue "access_token"))
      (set `self.refresh token` (`VaRestJsonObject.GetStringField` _returnvalue "refresh_token")))))

(event `RegisterTeam`
  (params (ID :type Integer64))
  ;[1 1 1] RegisterTeam
  (set `self.ID` ID)
  (bind _returnvalue (`VaRestSubsystem.ConstructVaRestRequestExt` (subsystem `VaRestSubsystem`) "POST" "json"))
  (bind _output_get (set `self.Json Post Object` _returnvalue))
  (add `VaRestRequestJSON.OnRequestComplete` _output_get (delegate `TeamRegistrated`))
  (add `VaRestRequestJSON.OnRequestFail` _output_get (delegate `FailToRegisterTeam`))
  (bind _returnvalue_2 (`VaRestRequestJSON.GetRequestObject` _output_get))
  (`VaRestJsonObject.SetBoolField` _returnvalue_2 "approved" true)
  (`VaRestJsonObject.SetStringField` _returnvalue_2 "teamName" (`self.TeamName`))
  (`VaRestJsonObject.SetStringField` _returnvalue_2 "skillLevel" "good")
  (`VaRestJsonObject.SetObjectField` _returnvalue_2 "contact" (`|MakeJson` (`self.FirstName`) (`self.Surename`) (`self.Email`) (`self.Phone Number`)))
  (`VaRestRequestJSON.ProcessURL` (`self.Json Post Object`) (`KismetStringLibrary.Concat_StrStr` (`self.URLPart1`) (`KismetTextLibrary.Conv_TextToString` (`KismetTextLibrary.Conv_Int64ToText` (`self.ID`))) (`self.URLPart2`))))

(event `FailToRegisterTeam`
  (params (Request :type "VaRestRequestJSON Object Reference"))
  ;[1 1 1] RegisterTeam
  (`KismetSystemLibrary.PrintString` "failed"))

(event `TeamRegistrated`
  (params (Request :type "VaRestRequestJSON Object Reference"))
  (bind _hudref (`self.HudRef`))
  (bind _tournament_info (`/Game/widgets/Tournament/MainHud.tournament_Info` _hudref))
  ;[1 1 1] RegisterTeam
  (`Widget.SetVisibility` (`/Game/widgets/Tournament/MainHud.RegisterTeam` _hudref) "Collapsed")
  (`Widget.SetVisibility` _tournament_info "Visible")
  (`/Game/widgets/Tournament/tournament_Info.RequestTournamentInfo` _tournament_info)
  (bind _returnvalue (`GameplayStatics.LoadGameFromSlot` "MyGame"))
  (bind _asmy_game (cast `/Game/Blueprints/MyGame` _returnvalue))
  (`KismetArrayLibrary.Array_Add` (`/Game/Blueprints/MyGame.myTournamentIDList` _asmy_game) (`VaRestRequestJSON.GetResponseObject` Request))
  (`AsyncActionHandleSaveGame.AsyncSaveGameToSlot` _asmy_game "MyGame"))

(event `RequestToRegisterTournament`
  (params (endDateAsISO8601 :type String) (startDateAsISO8601 :type String) (tournamentName :type String) (poolType :type String) (city :type String) (country :type String) (streetName :type String) (houseNumber :type String) (postalCode :type String) (pubDateAsISO8601 :type String) (id :type Integer64) (maxMatchTimeInSeconds :type Integer64) (numberOfPlaygrounds :type Integer64) (maxNumberOfParticipatingTeams :type Integer64))
  ;[0 0 0 1 50] Register Tournement
  (bind _output_get (set `self.End Date as ISO8601` endDateAsISO8601))
  (bind _output_get_2 (set `self.Start Date as ISO8601` startDateAsISO8601))
  (bind _output_get_3 (set `self.Tournament Name` tournamentName))
  (bind _output_get_4 (set `self.Pool Type` poolType))
  (bind _output_get_5 (set `self.City` city))
  (bind _output_get_6 (set `self.Country` country))
  (bind _output_get_7 (set `self.Street Name` streetName))
  (bind _output_get_8 (set `self.House Number` houseNumber))
  (bind _output_get_9 (set `self.Postal Code` postalCode))
  (bind _output_get_10 (set `self.Pub Date as ISO8601` pubDateAsISO8601))
  (set `self.Id_0` id)
  (bind _output_get_11 (set `self.Max Match Time in Seconds` maxMatchTimeInSeconds))
  (bind _output_get_12 (set `self.Number Of Playgrounds` numberOfPlaygrounds))
  (bind _output_get_13 (set `self.Max Number Of Participating Teams` maxNumberOfParticipatingTeams))
  (if (`KismetStringLibrary.IsEmpty` (`self.Bearer token`))
    (`Widget.SetVisibility` (`/Game/widgets/Tournament/MainHud.Select_LoginOrRegistrate` (`self.HudRef`)) "Visible")
    (else
      (bind _returnvalue (`VaRestSubsystem.ConstructVaRestRequestExt` (subsystem `VaRestSubsystem`) "POST" "json"))
      (`VaRestRequestJSON.SetHeader` _returnvalue "Authorization" (`KismetStringLibrary.Concat_StrStr` "Bearer " (`self.Bearer token`)))
      (add `VaRestRequestJSON.OnRequestComplete` _returnvalue (delegate `registerTournament`))
      (add `VaRestRequestJSON.OnRequestFail` _returnvalue (delegate `CustomEvent_3`))
      (bind _returnvalue_2 (`VaRestRequestJSON.GetRequestObject` _returnvalue))
      (`VaRestJsonObject.SetStringField` _returnvalue_2 "endDateAsISO8601" _output_get)
      ;;[1 1 1] set fields in Json Object
      (`VaRestJsonObject.SetStringField` _returnvalue_2 "startDateAsISO8601" _output_get_2)
      (`VaRestJsonObject.SetStringField` _returnvalue_2 "tournamentName" _output_get_3)
      (`VaRestJsonObject.SetStringField` _returnvalue_2 "poolType" _output_get_4)
      (`VaRestJsonObject.SetObjectField` _returnvalue_2 "location" (`|MakeJson` _output_get_5 _output_get_6 _output_get_7 _output_get_8 _output_get_9))
      (`VaRestJsonObject.SetStringField` _returnvalue_2 "pubDateAsISO8601" _output_get_10)
      (`VaRestJsonObject.SetInt64Field` _returnvalue_2 "maxMatchTimeInSeconds" _output_get_11)
      (`VaRestJsonObject.SetInt64Field` _returnvalue_2 "numberOfPlaygrounds" _output_get_12)
      (`VaRestJsonObject.SetInt64Field` _returnvalue_2 "maxNumberOfParticipatingTeams" _output_get_13)
      (`VaRestRequestJSON.ProcessURL` _returnvalue "http://localhost:8080/api/tournament/register"))))

(event `CustomEvent_3`
  (params (Request :type "VaRestRequestJSON Object Reference"))
  ;[0 0 0 1 50] Register Tournement
  (`KismetSystemLibrary.PrintString` "failed"))

(event `registerTournament`
  (params (Request :type "VaRestRequestJSON Object Reference"))
  (bind _returnvalue (`VaRestRequestJSON.GetResponseCode` Request))
  ;[0 0 0 1 50] Register Tournement
  (if (== _returnvalue 403)
    (`self.refreshToken` true)
    (elif (not (== _returnvalue 422))
      (bind _returnvalue_2 (`GameplayStatics.LoadGameFromSlot` "MyGame"))
      (bind _asmy_game (cast `/Game/Blueprints/MyGame` _returnvalue_2)))))

(event `refreshToken`
  (params (tournamentRegisration :type Boolean) (tournamentlist :type Boolean) (approvalstatus :type Boolean) (formTextfeld_ButtonRef :type "/Game/widgets/Tournament/approveField Object Reference"))
  ;[0 0 0] Refresh access token or show login screen is refrsh token expired
  ;;[1 1 1] create request
  (bind _returnvalue (`VaRestSubsystem.ConstructVaRestRequestExt` (subsystem `VaRestSubsystem`) "GET" "json"))
  (`VaRestRequestJSON.SetHeader` _returnvalue "Authorization" (`KismetStringLibrary.Concat_StrStr` "Bearer " (`self.refresh token`)))
  (add `VaRestRequestJSON.OnRequestComplete` _returnvalue (delegate `getNewToken`))
  (add `VaRestRequestJSON.OnRequestFail` _returnvalue (delegate `CustomEvent_1`))
  (`VaRestRequestJSON.ProcessURL` _returnvalue "http://localhost:8080/api/refresh-token"))

(event `CustomEvent_1`
  (params (Request :type "VaRestRequestJSON Object Reference"))
  ;[0 0 0] Refresh access token or show login screen is refrsh token expired
  ;;[1 1 1] create request
  (`KismetSystemLibrary.PrintString` "failed refresh tokken"))

(event `getNewToken`
  (params (Request :type "VaRestRequestJSON Object Reference"))
  (bind _returnvalue (`VaRestRequestJSON.GetResponseObject` Request))
  ;[0 0 0] Refresh access token or show login screen is refrsh token expired
  (bind _returnvalue_2 (`VaRestRequestJSON.GetResponseContentAsString` Request true))
  ;;[1 1 1] if token expired
  (if (`KismetStringLibrary.EqualEqual_StrStr` (`KismetStringLibrary.GetSubstring` _returnvalue_2 5 5) "error")
    ;;[1 1 1] create login screen
    (`Widget.SetVisibility` (`/Game/widgets/Tournament/MainHud.Select_LoginOrRegistrate` (`self.HudRef`)) "Visible")
    (else
      (set `self.Bearer token` (`VaRestJsonObject.GetStringField` _returnvalue "access_token"))
      (set `self.refresh token` (`VaRestJsonObject.GetStringField` _returnvalue "refresh_token"))
      (if (stale `refreshToken` tournamentRegisration)
        (`KismetSystemLibrary.PrintString` "refrehed token")
        ;;[1 1 1] get new bearer token and registrate tournament
        (`self.RequestToRegisterTournament` (`self.End Date as ISO8601`) (`self.Start Date as ISO8601`) (`self.Tournament Name`) (`self.Pool Type`) (`self.City`) (`self.Country`) (`self.Street Name`) (`self.House Number`) (`self.Postal Code`) (`self.Pub Date as ISO8601`) (`self.Id_0`) (`self.Max Match Time in Seconds`) (`self.Number Of Playgrounds`) (`self.Max Number Of Participating Teams`))
        (elif (stale `refreshToken` tournamentlist)
          (`/Game/widgets/Tournament/TournamentList.GetTournamentofPage` (`/Game/widgets/Tournament/MainHud.TournamentList` (`self.HudRef`)))
          (elif (stale `refreshToken` approvalstatus)
            (`/Game/widgets/Tournament/approveField.updateTeamStatus` (stale `refreshToken` formTextfeld_ButtonRef))))))))

(fn `UserConstructionScript`)