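; AR_Instance is the game instance blueprint that prepares the MyGame save slot on Init.
; It creates and saves a MyGame object if none exists, then loads the slot, sets its ReIniit flag and saves it back.
; An Android storage permission check is present but disconnected, and its grant callback runs the same save logic whether permission is granted or denied.
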(event `self.ReceiveInit`
  (bind _returnvalue (`GameplayStatics.DoesSaveGameExist` "MyGame" :!label _label))
  (if _returnvalue
    (bind _returnvalue_2 (`GameplayStatics.LoadGameFromSlot` "MyGame" :!label _label_2))
    (bind _asmy_game (cast `/Game/Blueprints/MyGame` _returnvalue_2))
    (set `/Game/Blueprints/MyGame.reIniit` true _asmy_game)
    (`GameplayStatics.SaveGameToSlot` _asmy_game "MyGame")
    (else
      (bind _returnvalue_3 (`GameplayStatics.CreateSaveGameObject` "/Game/Blueprints/MyGame.MyGame_C"))
      (bind _returnvalue_4 (`GameplayStatics.SaveGameToSlot` _returnvalue_3 "MyGame"))
      (if _returnvalue_4
        (goto _label_2)))))

(event `OnPermissionsGrantedDynamicDelegate_Event_0`
  (params (Permissions :type "Array of String (by ref)") (GrantResults :type "Array of Boolean (by ref)"))
  (if (`|GetArrayItem` GrantResults)
    (goto _label)
    (else
      (goto _label))))